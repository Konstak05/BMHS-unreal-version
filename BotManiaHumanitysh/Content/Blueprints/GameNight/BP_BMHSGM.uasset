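; Game manager for a timed night-survival mode with three enemy bots, closable doors, security cameras and win/lose screens.
; BeginPlay gathers actor references, starts the AI and UI, then runs looping one-second timers for night progress, battery and hour display.
; Each hour change refreshes the AI, and outlasting the final hour wins.
; Closed doors drain battery, charging requires all doors open, an empty battery opens them, and Tick syncs the camera ID.
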(event `Start Night Interval`
  (bind _nightinterval (`self.NightInterval`))
  (bind _nightinterval_2 (`self.NightInterval`))
  ;[1 0 0] StartNight
  (`/Engine/EditorBlueprintResources/StandardMacros.IncrementInt` _nightinterval
    (:`  `
      (`KismetSystemLibrary.PrintString` (`KismetStringLibrary.Conv_IntToString` _nightinterval))
      (switch `int` (`self.NightHour`)
        (:`0`
          (if (not (<= _nightinterval_2 29))
            (set `self.NightHour` 1)
            (`KismetSystemLibrary.PrintText` (`KismetTextLibrary.Conv_IntToText` (`self.NightHour`)) :!label _label)
            (`self.Refresh AI`)))
        (:`1`
          (if (not (<= _nightinterval_2 59))
            (set `self.NightHour` 2)
            (goto _label)))
        (:`2`
          (if (not (<= _nightinterval_2 99))
            (set `self.NightHour` 3)
            (goto _label)))
        (:`3`
          (if (not (<= _nightinterval_2 129))
            (set `self.NightHour` 4)
            (goto _label)))
        (:`4`
          (if (not (<= _nightinterval_2 149))
            (set `self.NightHour` 5)
            (goto _label)))
        (:`5`
          (if (not (<= _nightinterval_2 179))
            (`KismetSystemLibrary.PrintString` "You Win!")
            (`KismetSystemLibrary.K2_ClearAndInvalidateTimerHandle` (`self.StartNightTimerHandle`))
            (`KismetSystemLibrary.K2_ClearAndInvalidateTimerHandle` (`self.Battery Update Timer Handle`))
            (`KismetSystemLibrary.K2_ClearAndInvalidateTimerHandle` (`self.Hour Update Timer Handle`))
            (`self.StopAi`)
            (bind _returnvalue (`|CreateWidget` "/Game/Blueprints/GameNight/UI_BP/BM_YouWin.BM_YouWin_C"))
            (`UserWidget.AddToViewport` _returnvalue 0)))))))

(event `Battery Update Timer`
  ;[0 1 0] Battery System
  (`KismetSystemLibrary.PrintText` "BUT working!")
  (bind _output_get (set `self.BatteryCurrent` (`self.BatteryCurrent`)))
  (`/Game/Blueprints/GameNight/UI_BP/BP_GameNight_UI.UpdateCurrentBattery` (`self.GameNight UI Ref`) _output_get)
  (if (<= (`self.BatteryCurrent`) 0)
    (set `self.IsBatteryZero` true)
    (set `self.Door1closed` false)
    (set `self.Door2closed` false)
    (set `self.Door3closed` false)
    (`/Game/Blueprints/GameNight/BP_DoorSystem.Refresh Doors` (`self.DoorSystem`))
    (`KismetSystemLibrary.K2_ClearAndInvalidateTimerHandle` (`self.Battery Update Timer Handle`))
    (else
      (set `self.IsBatteryZero` false)
      (if (`self.Door1closed`)
        (`/Engine/EditorBlueprintResources/StandardMacros.DecrementInt` (`self.BatteryCurrent`)
          (:`  `
            _)))
      (if (`self.Door2closed`)
        (`/Engine/EditorBlueprintResources/StandardMacros.DecrementInt` (`self.BatteryCurrent`)
          (:`  `
            _)))
      (if (`self.Door3closed`)
        (`/Engine/EditorBlueprintResources/StandardMacros.DecrementInt` (`self.BatteryCurrent`)
          (:`  `
            _)))
      (if (`self.Door1closed`)
        _
        (elif (`self.Door2closed`)
          _
          (elif (`self.Door3closed`)
            _
            (elif (`self.IsCharging`)
              (if (<= (`self.BatteryCurrent`) 99)
                (bind _result (`/Engine/EditorBlueprintResources/StandardMacros.IncrementInt` (`self.BatteryCurrent`))
                  (:`  `
                    (`/Game/Blueprints/GameNight/UI_BP/BP_GameNight_UI.UpdateCurrentBattery` (`self.GameNight UI Ref`) _result)))))))))))

(event `self.ReceiveBeginPlay`
  ;[1 0 0.7359] Show Cursor and Get main camera
  (bind _returnvalue (`GameplayStatics.GetActorOfClass` "/Game/Blueprints/GameNight/BP_GameNight.BP_GameNight_C"))
  (bind _output_get (set `self.BPGameNight Ref` _returnvalue))
  (`PlayerController.SetViewTargetWithBlend` (`GameplayStatics.GetPlayerController` 0) _output_get 0.0 "VTBlend_Linear" 0.0 false)
  (set `PlayerController.bShowMouseCursor` true (`GameplayStatics.GetPlayerController` 0))
  ;[0 0.9271 1] Get Sec Camera Ref
  (bind _returnvalue_2 (`GameplayStatics.GetActorOfClass` "/Game/Blueprints/GameNight/BM_SecurityCamSystem.BM_SecurityCamSystem_C"))
  (set `self.BPSecCamSystem Ref` _returnvalue_2)
  ;[0 1 0.02598] Get Green Bot AI
  (bind _returnvalue_3 (`GameplayStatics.GetActorOfClass` "/Game/Blueprints/GameNight/EnemyAI.EnemyAI_C"))
  (set `self.EnemyAI1` _returnvalue_3)
  (`/Game/Blueprints/GameNight/EnemyAI.Start EnemyAI` (`self.EnemyAI1`))
  ;[0.1943 0 1] Get Blue Bot AI
  (bind _returnvalue_4 (`GameplayStatics.GetActorOfClass` "/Game/Blueprints/GameNight/EnemyAI2.EnemyAI2_C"))
  (set `self.EnemyAI2` _returnvalue_4)
  (`/Game/Blueprints/GameNight/EnemyAI2.Start EnemyAI2` (`self.EnemyAI2`))
  ;[1 0.01282 0] Get Red Bot AI
  (bind _returnvalue_5 (`GameplayStatics.GetActorOfClass` "/Game/Blueprints/GameNight/EnemyAI3.EnemyAI3_C"))
  (set `self.EnemyAI3` _returnvalue_5)
  (`/Game/Blueprints/GameNight/EnemyAI3.Start EnemyAI3` (`self.EnemyAI3`))
  ;[0 1 0.02598] DoorSystem
  (bind _returnvalue_6 (`GameplayStatics.GetActorOfClass` "/Game/Blueprints/GameNight/BP_DoorSystem.BP_DoorSystem_C"))
  (set `self.DoorSystem` _returnvalue_6)
  ;[1 0.07149 0] initialize everything
  (`self.BatteryInitialize `)
  (`self.Show GameNightUI`)
  (`KismetSystemLibrary.Delay` 2.0)
  ;[1 0 0] StartNight
  (bind _returnvalue_7 (`KismetSystemLibrary.K2_SetTimerDelegate` (delegate `Start Night Interval`) 1.0 true))
  (set `self.StartNightTimerHandle` _returnvalue_7)
  ;[0 1 0] Battery System
  (bind _returnvalue_8 (`KismetSystemLibrary.K2_SetTimerDelegate` (delegate `Battery Update Timer`) 1.0 true))
  (set `self.Battery Update Timer Handle` _returnvalue_8)
  ;[0.1277 0 1] Hour System
  (bind _returnvalue_9 (`KismetSystemLibrary.K2_SetTimerDelegate` (delegate `UpdateHour`) 1.0 true))
  (set `self.Hour Update Timer Handle` _returnvalue_9))

(event `Show GameNightUI`
  ;[1 1 0] Show User Interface
  (`/Engine/EditorBlueprintResources/StandardMacros.IsValid` (`self.GameNight UI Ref`)
    (:`Is Valid`
      _)
    (:`Is Not Valid`
      (bind _returnvalue (`|CreateWidget` "/Game/Blueprints/GameNight/UI_BP/BP_GameNight_UI.BP_GameNight_UI_C" null (`self.BPGameNight Ref`) (`self.BPSecCamSystem Ref`)))
      (set `self.GameNight UI Ref` _returnvalue)))
  (`UserWidget.AddToViewport` (`self.GameNight UI Ref`) 0))

(event `UpdateHour`
  ;[0.1277 0 1] Hour System
  (`KismetSystemLibrary.PrintText` "HUT working!")
  (bind _output_get (set `self.NightHour` (`self.NightHour`)))
  (`/Game/Blueprints/GameNight/UI_BP/BP_GameNight_UI.UpdateCurrentHour` (`self.GameNight UI Ref`) _output_get)
  (if (>= (`self.NightHour`) 6)
    (`KismetSystemLibrary.K2_ClearAndInvalidateTimerHandle` (`self.Hour Update Timer Handle`))))

(event `self.ReceiveTick`
  (params (DeltaSeconds :type "Float (single-precision)"))
  ;[0 0.8999 1] Set OpenCam ID to Cam System Ref
  (`/Engine/EditorBlueprintResources/StandardMacros.IsValid` (`self.BPSecCamSystem Ref`)
    (:`Is Valid`
      (set `/Game/Blueprints/GameNight/BM_SecurityCamSystem.CamID` (`self.CamOpenedID`) (`self.BPSecCamSystem Ref`))
      (if (< (`self.BatteryCurrent`) 0)
        (bind _output_get (set `self.BatteryCurrent` 0))
        (`/Game/Blueprints/GameNight/UI_BP/BP_GameNight_UI.UpdateCurrentBattery` (`self.GameNight UI Ref`) _output_get)))))

(event `GameOver`
  (`KismetSystemLibrary.K2_ClearAndInvalidateTimerHandle` (`self.StartNightTimerHandle`))
  (`KismetSystemLibrary.K2_ClearAndInvalidateTimerHandle` (`self.Battery Update Timer Handle`))
  (`KismetSystemLibrary.K2_ClearAndInvalidateTimerHandle` (`self.Hour Update Timer Handle`))
  (`self.StopAi`)
  (bind _returnvalue (`|CreateWidget` "/Game/Blueprints/GameNight/UI_BP/BM_YouLost.BM_YouLost_C"))
  (`UserWidget.AddToViewport` _returnvalue 0))

(event `StopAi`
  ;[0.1068 1 0] Green Bot
  (`/Game/Blueprints/GameNight/EnemyAI.Stop EnemyAI` (`self.EnemyAI1`))
  ;[0.2415 0 1] Blue Bot
  (`/Game/Blueprints/GameNight/EnemyAI2.Stop EnemyAI` (`self.EnemyAI2`))
  ;[1 0.007021 0] Red Bot
  (`/Game/Blueprints/GameNight/EnemyAI3.Stop EnemyAI` (`self.EnemyAI3`)))

(event `Refresh AI`
  ;[0.1068 1 0] Green Bot
  (`/Game/Blueprints/GameNight/EnemyAI.Refresh EnemyAI` (`self.EnemyAI1`))
  ;[0.2415 0 1] Blue Bot
  (`/Game/Blueprints/GameNight/EnemyAI2.Refresh EnemyAI2` (`self.EnemyAI2`))
  ;[1 0.007021 0] Red Bot
  (`/Game/Blueprints/GameNight/EnemyAI3.Refresh EnemyAI3` (`self.EnemyAI3`)))

(fn `BatteryInitialize `
  (set `self.BatteryCurrent` (`self.BatteryMax`)))

(fn `UserConstructionScript`)