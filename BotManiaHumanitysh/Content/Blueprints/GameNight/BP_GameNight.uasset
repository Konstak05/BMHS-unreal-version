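; BP_GameNight is an actor that turns left and right within a limited yaw arc, serving as the player movement for the game night.
; Start and stop events for each direction create and clear looping function-name timers, so no Tick logic is needed.
; Each timer calls LeftMovement or RightMovement, which checks the current yaw against that side's limit before adding a small world rotation step.
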(event `self.ReceiveBeginPlay`)

(event `self.ReceiveTick`
  (params (DeltaSeconds :type "Float (single-precision)")))

(event `StartMovementLeft`
  ;[1 0 0] PlayerMovement
  (bind _returnvalue (`KismetSystemLibrary.K2_SetTimer` null "LeftMovement" 0.03 true))
  (set `self.LeftMovementTimerHandle` _returnvalue))

(event `StopMovementLeft`
  ;[1 0 0] PlayerMovement
  (`KismetSystemLibrary.K2_ClearAndInvalidateTimerHandle` (`self.LeftMovementTimerHandle`)))

(event `StartMovementRight`
  ;[1 0 0] PlayerMovement
  (bind _returnvalue (`KismetSystemLibrary.K2_SetTimer` null "RightMovement" 0.03 true))
  (set `self.RightMovementTimerHandle` _returnvalue))

(event `StopMovementRight`
  ;[1 0 0] PlayerMovement
  (`KismetSystemLibrary.K2_ClearAndInvalidateTimerHandle` (`self.RightMovementTimerHandle`)))

(fn `LeftMovement`
  (bind (_returnvalue_roll _returnvalue_pitch _returnvalue_yaw) (`KismetMathLibrary.BreakRotator` (`self.K2_GetActorRotation`)))
  (if (>= _returnvalue_yaw -120.0)
    (`self.K2_AddActorWorldRotation` (`KismetMathLibrary.MakeRotator` 0.0 0.0 -1.5))))

(fn `RightMovement`
  (bind (_returnvalue_roll _returnvalue_pitch _returnvalue_yaw) (`KismetMathLibrary.BreakRotator` (`self.K2_GetActorRotation`)))
  (if (<= _returnvalue_yaw -60.0)
    (`self.K2_AddActorWorldRotation` (`KismetMathLibrary.MakeRotator` 0.0 0.0 1.5))))

(fn `UserConstructionScript`)