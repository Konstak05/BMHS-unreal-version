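; BP_DoorSystem shows or hides three door components to reflect the closed states stored in the BP_BMHSGM game mode.
; On BeginPlay it casts the game mode and sets each door visible when its closed flag is true, hidden otherwise.
; The RefreshDoors event reruns the same logic on demand, changing only visibility without propagating to child components.
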(event `self.ReceiveBeginPlay`
  (bind _door_2 (`self.Door 2`))
  (bind _door_3 (`self.Door 3`))
  (bind _door_1 (`self.Door 1`))
  (bind _asbp_bmhsgm (cast `/Game/Blueprints/GameNight/BP_BMHSGM` (`GameplayStatics.GetGameMode`) :!label _label))
  (if (`/Game/Blueprints/GameNight/BP_BMHSGM.Door1closed` _asbp_bmhsgm)
    (`SceneComponent.SetVisibility` _door_1 true false)
    (else
      (`SceneComponent.SetVisibility` _door_1 false false)))
  (if (`/Game/Blueprints/GameNight/BP_BMHSGM.Door2closed` _asbp_bmhsgm)
    (`SceneComponent.SetVisibility` _door_2 true false)
    (else
      (`SceneComponent.SetVisibility` _door_2 false false)))
  (if (`/Game/Blueprints/GameNight/BP_BMHSGM.Door3closed` _asbp_bmhsgm)
    (`SceneComponent.SetVisibility` _door_3 true false)
    (else
      (`SceneComponent.SetVisibility` _door_3 false false))))

(event `Refresh Doors`
  (goto _label))

(fn `UserConstructionScript`)