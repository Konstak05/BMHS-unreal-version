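; CCTV camera actor for the GameNight content that renders its view into a render target through a SceneCapture2D component.
; On BeginPlay it switches on its CamsID to assign one of ten CCTV render targets as the capture's texture target.
; Each camera instance therefore feeds its own feed texture, selected by ID.
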(event `self.ReceiveBeginPlay`
  (bind _scenecapturecomponent2d (`self.SceneCaptureComponent2D`))
  (switch `int` (`self.CamsID`)
    (:`0`
      (set `SceneCaptureComponent2D.TextureTarget` "/Game/RenderTargets/CCTV1.CCTV1" _scenecapturecomponent2d))
    (:`1`
      (set `SceneCaptureComponent2D.TextureTarget` "/Game/RenderTargets/CCTV2.CCTV2" _scenecapturecomponent2d))
    (:`2`
      (set `SceneCaptureComponent2D.TextureTarget` "/Game/RenderTargets/CCTV3.CCTV3" _scenecapturecomponent2d))
    (:`3`
      (set `SceneCaptureComponent2D.TextureTarget` "/Game/RenderTargets/CCTV4.CCTV4" _scenecapturecomponent2d))
    (:`4`
      (set `SceneCaptureComponent2D.TextureTarget` "/Game/RenderTargets/CCTV5.CCTV5" _scenecapturecomponent2d))
    (:`5`
      (set `SceneCaptureComponent2D.TextureTarget` "/Game/RenderTargets/CCTV6.CCTV6" _scenecapturecomponent2d))
    (:`6`
      (set `SceneCaptureComponent2D.TextureTarget` "/Game/RenderTargets/CCTV7.CCTV7" _scenecapturecomponent2d))
    (:`7`
      (set `SceneCaptureComponent2D.TextureTarget` "/Game/RenderTargets/CCTV8.CCTV8" _scenecapturecomponent2d))
    (:`8`
      (set `SceneCaptureComponent2D.TextureTarget` "/Game/RenderTargets/CCTV9.CCTV9" _scenecapturecomponent2d))
    (:`9`
      (set `SceneCaptureComponent2D.TextureTarget` "/Game/RenderTargets/CCTV10.CCTV10" _scenecapturecomponent2d))))

(fn `UserConstructionScript`)