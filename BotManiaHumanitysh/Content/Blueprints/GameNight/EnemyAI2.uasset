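; EnemyAI2 is the "Blue Bot" enemy, which creeps through six preset positions toward the player's Door 2.
; A looping four-second timer rolls a random move chance scaled by Difficulty (zero disables it), advancing the bot or, with CanBackTrack, stepping back from position 1.
; Movement is faked by showing one position component and hiding the rest.
; Moving from the last position resets it if BP_BMHSGM reports Door2closed, otherwise calls GameOver.
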(event `Start EnemyAI2`
  (`self.Refresh EnemyAI2`)
  (`KismetSystemLibrary.PrintText` "Blue Bot ready!")
  (`KismetSystemLibrary.Delay` 2.0)
  (bind _returnvalue (`KismetSystemLibrary.K2_SetTimerDelegate` (delegate `Active`) 4.0 true))
  (set `self.Active Enemy Timer Handle` _returnvalue)
  (`self.Refresh EnemyAI2`))

(event `Stop EnemyAI`
  (`KismetSystemLibrary.K2_ClearAndInvalidateTimerHandle` (`self.Active Enemy Timer Handle`)))

(event `Refresh EnemyAI2`
  (if (== (`self.Difficulty`) 0)
    (`self.Stop EnemyAI`)
    (else
      (set `self.EnemyWalkMax` (/ 20 (`self.Difficulty`)))))
  (switch `int` (`self.EnemyPosition`)
    (:`0`
      (`SceneComponent.SetVisibility` (`self.Position4`) false false)
      (`SceneComponent.SetVisibility` (`self.Position2`) false false)
      (`SceneComponent.SetVisibility` (`self.Position3`) false false)
      (`SceneComponent.SetVisibility` (`self.Position5`) false false)
      (`SceneComponent.SetVisibility` (`self.Position6`) false false)
      (`SceneComponent.SetVisibility` (`self.Position1`) true false))))

(event `Active`
  (bind _enemyposition (`self.EnemyPosition`))
  ;[1 1 1] EnemyAIActive
  (`KismetSystemLibrary.PrintString` "Blue Bot Interval")
  (set `self.WalkOpportunity` (`KismetMathLibrary.RandomIntegerInRange` 0 (`self.EnemyWalkMax`)))
  (switch `int` (`self.WalkOpportunity`)
    (:`0`
      (if (`self.CanBackTrack`)
        (switch `int` _enemyposition
          (:`1`
            (bind _result (`/Engine/EditorBlueprintResources/StandardMacros.DecrementInt` _enemyposition)
              (:`  `
                (set `self.EnemyPosition` _result)
                (switch `int` _enemyposition :!label _label
                  (:`0`
                    (`SceneComponent.SetVisibility` (`self.Position4`) false false)
                    (`SceneComponent.SetVisibility` (`self.Position2`) false false)
                    (`SceneComponent.SetVisibility` (`self.Position3`) false false)
                    (`SceneComponent.SetVisibility` (`self.Position5`) false false)
                    (`SceneComponent.SetVisibility` (`self.Position6`) false false)
                    (`SceneComponent.SetVisibility` (`self.Position1`) true false))
                  (:`1`
                    (`SceneComponent.SetVisibility` (`self.Position4`) false false)
                    (`SceneComponent.SetVisibility` (`self.Position3`) false false)
                    (`SceneComponent.SetVisibility` (`self.Position5`) false false)
                    (`SceneComponent.SetVisibility` (`self.Position6`) false false)
                    (`SceneComponent.SetVisibility` (`self.Position1`) false false)
                    (`SceneComponent.SetVisibility` (`self.Position2`) true false))
                  (:`2`
                    (`SceneComponent.SetVisibility` (`self.Position4`) false false)
                    (`SceneComponent.SetVisibility` (`self.Position2`) false false)
                    (`SceneComponent.SetVisibility` (`self.Position5`) false false)
                    (`SceneComponent.SetVisibility` (`self.Position6`) false false)
                    (`SceneComponent.SetVisibility` (`self.Position1`) false false)
                    (`SceneComponent.SetVisibility` (`self.Position3`) true false))
                  (:`3`
                    (`SceneComponent.SetVisibility` (`self.Position2`) false false)
                    (`SceneComponent.SetVisibility` (`self.Position3`) false false)
                    (`SceneComponent.SetVisibility` (`self.Position5`) false false)
                    (`SceneComponent.SetVisibility` (`self.Position6`) false false)
                    (`SceneComponent.SetVisibility` (`self.Position1`) false false)
                    (`SceneComponent.SetVisibility` (`self.Position4`) true false))
                  (:`4`
                    (`SceneComponent.SetVisibility` (`self.Position4`) false false)
                    (`SceneComponent.SetVisibility` (`self.Position2`) false false)
                    (`SceneComponent.SetVisibility` (`self.Position3`) false false)
                    (`SceneComponent.SetVisibility` (`self.Position6`) false false)
                    (`SceneComponent.SetVisibility` (`self.Position1`) false false)
                    (`SceneComponent.SetVisibility` (`self.Position5`) true false))
                  (:`5`
                    (`SceneComponent.SetVisibility` (`self.Position4`) false false)
                    (`SceneComponent.SetVisibility` (`self.Position2`) false false)
                    (`SceneComponent.SetVisibility` (`self.Position3`) false false)
                    (`SceneComponent.SetVisibility` (`self.Position5`) false false)
                    (`SceneComponent.SetVisibility` (`self.Position1`) false false)
                    (`SceneComponent.SetVisibility` (`self.Position6`) true false)))))))
        (else
          (switch `int` _enemyposition :!label _label_2
            (:`0`
              (bind _result_2 (`/Engine/EditorBlueprintResources/StandardMacros.IncrementInt` _enemyposition :!label _label_3)
                (:`  `
                  (set `self.EnemyPosition` _result_2)
                  (goto _label))))
            (:`1`
              (goto _label_3))
            (:`2`
              (goto _label_3))
            (:`3`
              (goto _label_3))
            (:`4`
              (goto _label_3))
            (:`5`
              (bind _asbp_bmhsgm (cast `/Game/Blueprints/GameNight/BP_BMHSGM` (`GameplayStatics.GetGameMode`)))
              (if (`/Game/Blueprints/GameNight/BP_BMHSGM.Door2closed` _asbp_bmhsgm)
                (set `self.EnemyPosition` 0)
                (goto _label)
                (else
                  (`/Game/Blueprints/GameNight/BP_BMHSGM.GameOver` _asbp_bmhsgm))))))))
    (:`1`
      (goto _label_2))))

(fn `Refresh EnemyAI`)

(fn `UserConstructionScript`)