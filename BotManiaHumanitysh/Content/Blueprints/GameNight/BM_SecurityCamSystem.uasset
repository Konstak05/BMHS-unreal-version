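; Security camera monitor actor that flips open and closed and displays one of ten CCTV screens.
; Each Tick it steps the actor's roll toward one of two end angles depending on IsOpened.
; Once that limit is reached, in either state, it switches on CamID every frame to set the matching CCTV material on Camera1.
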(event `self.ReceiveBeginPlay`)

(event `self.ReceiveTick`
  (params (DeltaSeconds :type "Float (single-precision)"))
  (bind _returnvalue_roll (`KismetMathLibrary.BreakRotator` (`self.K2_GetActorRotation`)))
  (bind _returnvalue_roll_2 (`KismetMathLibrary.BreakRotator` (`self.K2_GetActorRotation`)))
  ;[1 0.004897 0] CameraRotation
  (if (== (`self.IsOpened`) false)
    (if (>= _returnvalue_roll -175.0)
      (`self.K2_AddActorWorldRotation` (`KismetMathLibrary.MakeRotator` -3.0))
      (else
        ;[0.1351 0 1] Camera System Screens
        (switch `int` (`self.CamID`) :!label _label
          (:`0`
            (bind _output_get (set `self.Camera1` (`self.Camera1`)))
            (`PrimitiveComponent.SetMaterial` _output_get 0 "/Game/RenderTargets/CCTV1_Mat.CCTV1_Mat"))
          (:`1`
            (bind _output_get_2 (set `self.Camera1` (`self.Camera1`)))
            (`PrimitiveComponent.SetMaterial` _output_get_2 0 "/Game/RenderTargets/CCTV2_Mat.CCTV2_Mat"))
          (:`2`
            (bind _output_get_3 (set `self.Camera1` (`self.Camera1`)))
            (`PrimitiveComponent.SetMaterial` _output_get_3 0 "/Game/RenderTargets/CCTV3_Mat.CCTV3_Mat"))
          (:`3`
            (bind _output_get_4 (set `self.Camera1` (`self.Camera1`)))
            (`PrimitiveComponent.SetMaterial` _output_get_4 0 "/Game/RenderTargets/CCTV4_Mat.CCTV4_Mat"))
          (:`4`
            (bind _output_get_5 (set `self.Camera1` (`self.Camera1`)))
            (`PrimitiveComponent.SetMaterial` _output_get_5 0 "/Game/RenderTargets/CCTV5_Mat.CCTV5_Mat"))
          (:`5`
            (bind _output_get_6 (set `self.Camera1` (`self.Camera1`)))
            (`PrimitiveComponent.SetMaterial` _output_get_6 0 "/Game/RenderTargets/CCTV6_Mat.CCTV6_Mat"))
          (:`6`
            (bind _output_get_7 (set `self.Camera1` (`self.Camera1`)))
            (`PrimitiveComponent.SetMaterial` _output_get_7 0 "/Game/RenderTargets/CCTV7_Mat.CCTV7_Mat"))
          (:`7`
            (bind _output_get_8 (set `self.Camera1` (`self.Camera1`)))
            (`PrimitiveComponent.SetMaterial` _output_get_8 0 "/Game/RenderTargets/CCTV8_Mat.CCTV8_Mat"))
          (:`8`
            (bind _output_get_9 (set `self.Camera1` (`self.Camera1`)))
            (`PrimitiveComponent.SetMaterial` _output_get_9 0 "/Game/RenderTargets/CCTV9_Mat.CCTV9_Mat"))
          (:`9`
            (bind _output_get_10 (set `self.Camera1` (`self.Camera1`)))
            (`PrimitiveComponent.SetMaterial` _output_get_10 0 "/Game/RenderTargets/CCTV10_Mat.CCTV10_Mat")))))
    (elif (<= _returnvalue_roll_2 0.0)
      (`self.K2_AddActorWorldRotation` (`KismetMathLibrary.MakeRotator` 3.0))
      (else
        (goto _label)))))

(fn `UserConstructionScript`)